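; DrawPredictedObjects is an actor with a bounding box, apparently meant as a short-lived marker for predicted objects.
; Its Spawn event scales BoundingBox to Size, then spawns another DrawPredictedObjects actor at SpawnTransform.
; Tick counts DecayTime down, but the branch that destroys the actor at zero is unconnected, as is an empty check on Request, so nothing here removes the actor.
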(event Custom|Spawn
  (Transformation|SetWorldScale3D (Variables|Default|GetBoundingBox) (Variables|Default|Getsize))
  (Game|SpawnActorfromClass "DrawPredictedObjects_C" (Variables|Default|GetSpawn%20Transform) "Undefined" 0 0))

(event EventTick
  (params (DeltaSeconds :type Float%20%28single-precision%29))
  (bind _output_get (Variables|Default|Setdecay%20time (- (Variables|Default|Getdecay%20time) DeltaSeconds))))

(fn ConstructionScript)