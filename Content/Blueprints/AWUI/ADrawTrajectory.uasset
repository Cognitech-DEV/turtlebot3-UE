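; Actor that visualizes a trajectory received as a ROS 2 Path message through a node it initializes on BeginPlay.
; Each message resets the dynamic mesh and converts poses to Unreal transforms, scaling to centimeters, flipping Y and negating the rotator.
; Geometry Script sweeps the TrajShape polyline along those transforms, then remaps the material ID to show the trajectory material.
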(event Custom|Callback
  (params (InMessage :type ROS2%20Generic%20Msg%20Object%20Reference))
  (bind _traj (Variables|Default|Gettraj))
  (bind _asros2path_msg (Utilities|Casting|CastToROS2PathMsg InMessage))
  (bind _returnvalue (DynamicMeshComponent|GetDynamicMesh (Variables|DynamicMeshActor|GetDynamicMeshComponent)))
  (DynamicMesh|Reset _returnvalue)
  (Utilities|Array|Clear _traj)
  (for _array_element (.Poses (Utilities|Struct|BreakROSPath (Class|ROS2PathMsg|GetMsg _asros2path_msg)))
    (Utilities|Array|Add _traj (Math|Transform|MakeTransform (* (.Position (Utilities|Struct|BreakROSPose (.Pose (Utilities|Struct|BreakROSPoseStamped _array_element)))) "100.000000,-100.000000,100.000000") (* (Class|KismetMathLibrary|QuatRotator (.Orientation (Utilities|Struct|BreakROSPose (.Pose (Utilities|Struct|BreakROSPoseStamped _array_element))))) -1.0))))
  (bind _returnvalue_2 (GeometryScript|Primitives|AppendSweepPolyline :TargetMesh _returnvalue :PolylineVertices (Variables|Default|Gettraj_shape) :SweepPath _traj :Debug 0))
  (GeometryScript|Materials|RemapMaterialIDs _returnvalue_2 0 1 0)
  (Rendering|Material|SetMaterial (Variables|DynamicMeshActor|GetDynamicMeshComponent) 1 "/Game/Blueprints/AWUI/MTrajectory.MTrajectory"))

(event EventBeginPlay
  (bind _ros2subscriber (Variables|Default|GetROS2Subscriber))
  (bind _ros2node (Variables|Default|GetROS2Node))
  (bind _subscriber (Variables|/Script/rclUE.ROS2SubscriberComponent|GetSubscriber _ros2subscriber))
  (Class|ROS2NodeComponent|Init _ros2node)
  (Class|ROS2Subscriber|SetDelegates _subscriber (delegate Custom|Callback))
  (Class|ROS2NodeComponent|AddSubscription _ros2node _subscriber))

(fn ConstructionScript)