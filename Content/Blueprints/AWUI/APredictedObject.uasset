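; APredictedObject is an actor that represents a predicted object with a bounding box, candidate paths and a limited lifetime.
; Spawn scales the bounding box by Size and spawns another APredictedObject at SpawnTransform, while Tick counts DecayTime down and destroys the actor at zero.
; Updated moves it to SpawnTransform and draws each predicted path as 2D line segments tinted by confidence, using an empty paint context.
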(event Custom|Updated
  (Transformation|SetActorTransform (Variables|Default|GetSpawn%20Transform))
  (for _array_element (Variables|Default|Getpredicted%20path)
    (for (_array_element_2 _array_index) (.Path (Utilities|Struct|BreakROSPredictedPath _array_element))
      (if (> _array_index 0)
        (Class|WidgetBlueprintLibrary|DrawLine (Utilities|Struct|MakePaintContext) (Math|Conversions|ToVector2D(Vector) (.Position (Utilities|Struct|BreakROSPose (Utilities|Array|Get(acopy) (.Path (Utilities|Struct|BreakROSPredictedPath _array_element)) (- _array_index 1))))) (Math|Conversions|ToVector2D(Vector) (.Position (Utilities|Struct|BreakROSPose _array_element_2))) (Math|Conversions|ToLinearColor(Float) (.Confidence (Utilities|Struct|BreakROSPredictedPath _array_element))))))))

(event Custom|Spawn
  (Transformation|SetWorldScale3D (Variables|Default|GetBoundingBox) (Variables|Default|Getsize))
  (Game|SpawnActorfromClass "APredictedObject_C" (Variables|Default|GetSpawn%20Transform) "Undefined" 0 0))

(event EventTick
  (params (DeltaSeconds :type Float%20%28single-precision%29))
  (bind _output_get (Variables|Default|Setdecay%20time (- (Variables|Default|Getdecay%20time) DeltaSeconds)))
  (if (<= _output_get 0.0)
    (Actor|DestroyActor)))

(fn ConstructionScript)