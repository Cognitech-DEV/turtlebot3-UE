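; ROS 2 node actor that displays a raw image feed on a plate and follows the received ego pose.
; On BeginPlay it initializes DrawImageNode and registers the image and pose subscriptions.
; Pose messages move the actor, scaling metres to centimetres, flipping Y, adding a height offset and negating the rotator.
; Image messages are converted to textures and fed to the plate through a dynamic material instance created per message.
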(event Custom|ImageCB
  (params (InMessage :type ROS2%20Generic%20Msg%20Object%20Reference))
  (bind _asros2img_msg (Utilities|Casting|CastToROS2ImgMsg InMessage))
  (bind _returnvalue (Class|ROS2ImgtoTexture|Convert (Class|ROS2ImgMsg|GetMsg _asros2img_msg)))
  (bind _returnvalue_2 (Rendering|Material|CreateDynamicMaterialInstance (Variables|Default|GetAWUIImagePlate) 0 0 "None" :!class /Script/Engine.PrimitiveComponent))
  (Rendering|Material|SetTextureParameterValue _returnvalue_2 "InputTexture" _returnvalue))

(event Custom|PoseCB
  (params (InMessage :type ROS2%20Generic%20Msg%20Object%20Reference))
  (bind _asros2pose_stamped_msg (Utilities|Casting|CastToROS2PoseStampedMsg InMessage))
  (Transformation|SetActorTransform (Math|Transform|MakeTransform (+ (* (.Position (Utilities|Struct|BreakROSPose (.Pose (Utilities|Struct|BreakROSPoseStamped (Class|ROS2PoseStampedMsg|GetMsg _asros2pose_stamped_msg))))) "100.000000,-100.000000,100.000000") "0.000000,0.000000,100.000000") (* (Class|KismetMathLibrary|QuatRotator (.Orientation (Utilities|Struct|BreakROSPose (.Pose (Utilities|Struct|BreakROSPoseStamped (Class|ROS2PoseStampedMsg|GetMsg _asros2pose_stamped_msg)))))) -1.0))))

(event EventBeginPlay
  (bind _drawimagenode (Variables|Default|GetDrawImageNode))
  (bind _subimageraw (Variables|Default|GetSubImageRaw))
  (bind _subegopose (Variables|Default|GetSubEgoPose))
  (bind _subscriber (Variables|/Script/rclUE.ROS2SubscriberComponent|GetSubscriber _subimageraw))
  (bind _subscriber_2 (Variables|/Script/rclUE.ROS2SubscriberComponent|GetSubscriber _subegopose))
  (Class|ROS2NodeComponent|Init _drawimagenode)
  (Class|ROS2Subscriber|SetDelegates _subscriber (delegate Custom|ImageCB))
  (Class|ROS2NodeComponent|AddSubscription _drawimagenode _subscriber)
  (Class|ROS2Subscriber|SetDelegates _subscriber_2 (delegate Custom|PoseCB))
  (Class|ROS2NodeComponent|AddSubscription _drawimagenode _subscriber_2))

(fn ConstructionScript)