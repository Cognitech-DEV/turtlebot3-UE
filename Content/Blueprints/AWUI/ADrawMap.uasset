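; ADrawMap is a generated dynamic mesh actor meant to draw a map from ROS 2 marker array messages.
; DrawMapNode subscribes through SubMapMarker and passes triangle-list markers (type 11) to DrawTriangle.
; DrawTriangle appends vertices and builds index triples, but its triangle-creation nodes are disconnected, so no faces are added.
; Mesh rebuild separately creates a hard-coded test quad using the MTrajectory material.
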(event Custom|MapMarkerCB
  (params (InMessage :type ROS2%20Generic%20Msg%20Object%20Reference))
  (bind _asros2marker_array_msg (Utilities|Casting|CastToROS2MarkerArrayMsg InMessage))
  (for _array_element (Utilities|Struct|BreakROSMarkerArray (Class|ROS2MarkerArrayMsg|GetMsg _asros2marker_array_msg))
    (switch int (.Type (Utilities|Struct|BreakROSMarker _array_element))
      (:11
        (CallFunction|DrawTriangle (.Points (Utilities|Struct|BreakROSMarker _array_element)) (.Colors (Utilities|Struct|BreakROSMarker _array_element)))))))

(event EventBeginPlay
  (bind _drawmapnode (Variables|Default|GetDrawMapNode))
  (bind _submapmarker (Variables|Default|GetSubMapMarker))
  (bind _subscriber (Variables|/Script/rclUE.ROS2SubscriberComponent|GetSubscriber _submapmarker))
  (Class|ROS2NodeComponent|Init _drawmapnode)
  (Class|ROS2Subscriber|SetDelegates _subscriber (delegate Custom|MapMarkerCB))
  (Class|ROS2NodeComponent|AddSubscription _drawmapnode _subscriber))

(event Events|EventOnRebuildGeneratedMesh
  (params (TargetMesh :type Dynamic%20Mesh%20Object%20Reference))
  (bind _vectorlist (GeometryScript|ListUtils|ConvertArraytoVectorList (Utilities|Array|MakeArray "0, 0, 0" "100.000000,0.000000,0.000000" "0.000000,100.000000,0.000000" "100.000000,100.000000,0.000000")))
  (bind _returnvalue (GeometryScript|MeshEdits|AddVerticestoMesh TargetMesh _vectorlist))
  (bind _trianglelist (Class|GeometryScriptLibraryListUtilityFunctions|ConvertArraytoTriangleList (Utilities|Array|MakeArray (Utilities|Struct|MakeIntVector 0 2 1) (Utilities|Struct|MakeIntVector 1 2 3))))
  (bind (_newindiceslist _returnvalue_2) (Class|GeometryScriptLibraryMeshBasicEditFunctions|AddTrianglestoMesh _returnvalue _trianglelist 1 false 0))
  (GeometryScript|Materials|SetMaterialIDOnTriangles _returnvalue_2 _newindiceslist 1 false 0)
  (Rendering|Material|SetMaterial (Variables|DynamicMeshActor|GetDynamicMeshComponent) 1 "/Game/Blueprints/AWUI/MTrajectory.MTrajectory"))

(fn ConstructionScript)

(fn DrawTriangle
  (params (points :type Array%20of%20Vectors) (colors :type Array%20of%20ROS%20Color%20RGBA%20Structures))
  (Utilities|Array|Clear (LocalVariables|GetTriangle%20List))
  (bind _returnvalue (DynamicMeshComponent|GetDynamicMesh (Variables|DynamicMeshActor|GetDynamicMeshComponent)))
  (bind _vectorlist (GeometryScript|ListUtils|ConvertArraytoVectorList points))
  (bind (_newindiceslist _returnvalue_2) (GeometryScript|MeshEdits|AddVerticestoMesh _returnvalue _vectorlist))
  (bind _indexarray (Class|GeometryScriptLibraryListUtilityFunctions|ConvertIndexListtoArray _newindiceslist))
  (for (_ _array_index) _indexarray
    (if (== (Math|Integer|%(Integer) _array_index 3) 0)
      (Utilities|Array|Add (LocalVariables|GetTriangle%20List) (Utilities|Struct|MakeIntVector _array_index (+ _array_index 1) (+ _array_index 2)))))
  (Rendering|Material|SetMaterial (Variables|DynamicMeshActor|GetDynamicMeshComponent) 1 "/Game/Blueprints/AWUI/MTrajectory.MTrajectory"))