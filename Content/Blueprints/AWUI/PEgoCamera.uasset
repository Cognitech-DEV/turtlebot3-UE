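; PEgoCamera is an actor, apparently an ego camera, whose transform follows pose messages received over ROS 2.
; On BeginPlay it initializes a ROS 2 node and registers a PoseStamped subscriber with PoseCB as the callback.
; Each message sets the actor transform, converting to Unreal's left-handed centimeters by scaling position with Y flipped and negating quaternion X and Z.
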(event Custom|PoseCB
  (params (InMessage :type ROS2%20Generic%20Msg%20Object%20Reference))
  (bind _asros2pose_stamped_msg (Utilities|Casting|CastToROS2PoseStampedMsg InMessage))
  (Transformation|SetActorTransform (Math|Transform|MakeTransform (* (.Position (Utilities|Struct|BreakROSPose (.Pose (Utilities|Struct|BreakROSPoseStamped (Class|ROS2PoseStampedMsg|GetMsg _asros2pose_stamped_msg))))) "100.000000,-100.000000,100.000000") (Class|KismetMathLibrary|QuatRotator (Class|KismetMathLibrary|MakeQuat (* (.X (Class|KismetMathLibrary|BreakQuat (.Orientation (Utilities|Struct|BreakROSPose (.Pose (Utilities|Struct|BreakROSPoseStamped (Class|ROS2PoseStampedMsg|GetMsg _asros2pose_stamped_msg))))))) -1.0) (.Y (Class|KismetMathLibrary|BreakQuat (.Orientation (Utilities|Struct|BreakROSPose (.Pose (Utilities|Struct|BreakROSPoseStamped (Class|ROS2PoseStampedMsg|GetMsg _asros2pose_stamped_msg))))))) (* (.Z (Class|KismetMathLibrary|BreakQuat (.Orientation (Utilities|Struct|BreakROSPose (.Pose (Utilities|Struct|BreakROSPoseStamped (Class|ROS2PoseStampedMsg|GetMsg _asros2pose_stamped_msg))))))) -1.0) (.W (Class|KismetMathLibrary|BreakQuat (.Orientation (Utilities|Struct|BreakROSPose (.Pose (Utilities|Struct|BreakROSPoseStamped (Class|ROS2PoseStampedMsg|GetMsg _asros2pose_stamped_msg))))))))))))

(event EventBeginPlay
  (bind _ros2nodepose (Variables|Default|GetROS2NodePose))
  (bind _ros2subscriberpose (Variables|Default|GetROS2SubscriberPose))
  (bind _subscriber (Variables|/Script/rclUE.ROS2SubscriberComponent|GetSubscriber _ros2subscriberpose))
  (Class|ROS2NodeComponent|Init _ros2nodepose)
  (Class|ROS2Subscriber|SetDelegates _subscriber (delegate Custom|PoseCB))
  (Class|ROS2NodeComponent|AddSubscription _ros2nodepose _subscriber))

(event Collision|EventActorBeginOverlap
  (params (OtherActor :type Actor%20Object%20Reference)))

(event EventTick
  (params (DeltaSeconds :type Float%20%28single-precision%29)))

(fn ConstructionScript)