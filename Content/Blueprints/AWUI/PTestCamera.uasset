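; PTestCamera is a test camera actor whose transform is driven by ROS 2 PoseStamped messages.
; On BeginPlay it initializes a ROS 2 node and registers a subscriber with a callback.
; The callback moves the actor to each received pose, scaling position by 100 with Y flipped and negating every component of the quaternion-derived rotator.
; A position debug print is left unconnected.
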(event Custom|callback
  (params (InMessage :type ROS2%20Generic%20Msg%20Object%20Reference))
  (bind _asros2pose_stamped_msg (Utilities|Casting|CastToROS2PoseStampedMsg InMessage))
  (Transformation|SetActorTransform (Math|Transform|MakeTransform (* (.Position (Utilities|Struct|BreakROSPose (.Pose (Utilities|Struct|BreakROSPoseStamped (Class|ROS2PoseStampedMsg|GetMsg _asros2pose_stamped_msg))))) "100.000000,-100.000000,100.000000") (* (Class|KismetMathLibrary|QuatRotator (.Orientation (Utilities|Struct|BreakROSPose (.Pose (Utilities|Struct|BreakROSPoseStamped (Class|ROS2PoseStampedMsg|GetMsg _asros2pose_stamped_msg)))))) -1.0))))

(event EventBeginPlay
  (bind _ros2subscriber (Variables|Default|GetROS2Subscriber))
  (bind _ros2node (Variables|Default|GetROS2Node))
  (bind _subscriber (Variables|/Script/rclUE.ROS2SubscriberComponent|GetSubscriber _ros2subscriber))
  (Class|ROS2NodeComponent|Init _ros2node)
  (Class|ROS2Subscriber|SetDelegates _subscriber (delegate Custom|callback))
  (Class|ROS2NodeComponent|AddSubscription _ros2node _subscriber))

(fn ConstructionScript)