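; Actor that mirrors ROS2 predicted-object messages in the level through APredictedObject actors.
; BeginPlay starts a ROS2 node and subscription whose callback looks up each object by converted ID in a map.
; Known objects get a new pose and predicted paths; unknown ones also get a size, then Spawn and a map entry.
; Tick decrements each object's DecayTime per frame and destroys expired actors without removing their map entries.
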(event Custom|Callback
  (params (InMessage :type ROS2%20Generic%20Msg%20Object%20Reference))
  (bind _objects (Variables|Default|GetObjects))
  (bind _asros2predicted_objects_msg (Utilities|Casting|CastToROS2PredictedObjectsMsg InMessage))
  (for _array_element (.Objects (Utilities|Struct|BreakROSPredictedObjects (Class|ROS2PredictedObjectsMsg|GetMsg _asros2predicted_objects_msg)))
    (bind _returnvalue (Class|UuidtoString|Convert (.ObjectId (Utilities|Struct|BreakROSPredictedObject _array_element))))
    (if (.ReturnValue (Utilities|Map|Find _objects _returnvalue))
      (Variables|/Game/Blueprints/AWUI/APredictedObject.APredictedObject_C|SetSpawn%20Transform (.Value (Utilities|Map|Find _objects _returnvalue)) (Math|Transform|MakeTransform (.Position (Utilities|Struct|BreakROSPose (.Pose (Utilities|Struct|BreakROSPoseCov (.InitialPoseWithCovariance (Utilities|Struct|BreakROSPredictedObjectKinematics (.Kinematics (Utilities|Struct|BreakROSPredictedObject _array_element)))))))) (Class|KismetMathLibrary|QuatRotator (.Orientation (Utilities|Struct|BreakROSPose (.Pose (Utilities|Struct|BreakROSPoseCov (.InitialPoseWithCovariance (Utilities|Struct|BreakROSPredictedObjectKinematics (.Kinematics (Utilities|Struct|BreakROSPredictedObject _array_element)))))))))))
      (Variables|/Game/Blueprints/AWUI/APredictedObject.APredictedObject_C|Setpredicted%20path (.Value (Utilities|Map|Find _objects _returnvalue)) (.PredictedPaths (Utilities|Struct|BreakROSPredictedObjectKinematics (.Kinematics (Utilities|Struct|BreakROSPredictedObject _array_element)))))
      (Default|Updated (.Value (Utilities|Map|Find _objects _returnvalue)))
      (else
        (bind _returnvalue_2 (Actor|GetActorOfClass "/Game/Blueprints/AWUI/APredictedObject.APredictedObject_C"))
        (Variables|/Game/Blueprints/AWUI/APredictedObject.APredictedObject_C|Setsize _returnvalue_2 (.Dimensions (Utilities|Struct|BreakROSShape (.Shape (Utilities|Struct|BreakROSPredictedObject _array_element)))))
        (Variables|/Game/Blueprints/AWUI/APredictedObject.APredictedObject_C|SetSpawn%20Transform _returnvalue_2 (Math|Transform|MakeTransform (.Position (Utilities|Struct|BreakROSPose (.Pose (Utilities|Struct|BreakROSPoseCov (.InitialPoseWithCovariance (Utilities|Struct|BreakROSPredictedObjectKinematics (.Kinematics (Utilities|Struct|BreakROSPredictedObject _array_element)))))))) (Class|KismetMathLibrary|QuatRotator (.Orientation (Utilities|Struct|BreakROSPose (.Pose (Utilities|Struct|BreakROSPoseCov (.InitialPoseWithCovariance (Utilities|Struct|BreakROSPredictedObjectKinematics (.Kinematics (Utilities|Struct|BreakROSPredictedObject _array_element)))))))))))
        (Variables|/Game/Blueprints/AWUI/APredictedObject.APredictedObject_C|Setpredicted%20path _returnvalue_2 (.PredictedPaths (Utilities|Struct|BreakROSPredictedObjectKinematics (.Kinematics (Utilities|Struct|BreakROSPredictedObject _array_element)))))
        (Default|Spawn _returnvalue_2)
        (Utilities|Map|Add _objects _returnvalue 0)))))

(event EventBeginPlay
  (bind _subpredictedobjects (Variables|Default|GetSubPredictedObjects))
  (bind _predictedobjectsnode (Variables|Default|GetPredictedObjectsNode))
  (bind _subscriber (Variables|/Script/rclUE.ROS2SubscriberComponent|GetSubscriber _subpredictedobjects))
  (Class|ROS2NodeComponent|Init _predictedobjectsnode)
  (Class|ROS2Subscriber|SetDelegates _subscriber (delegate Custom|Callback))
  (Class|ROS2NodeComponent|AddSubscription _predictedobjectsnode _subscriber))

(event EventTick
  (params (DeltaSeconds :type Float%20%28single-precision%29))
  (bind _values (Utilities|Map|Values (Variables|Default|GetObjects)))
  (for _array_element _values
    (if (<= (Variables|/Game/Blueprints/AWUI/APredictedObject.APredictedObject_C|Getdecay%20time _array_element) 0.0)
      (Actor|DestroyActor _array_element)
      (else
        (Variables|/Game/Blueprints/AWUI/APredictedObject.APredictedObject_C|Setdecay%20time _array_element (- (Variables|/Game/Blueprints/AWUI/APredictedObject.APredictedObject_C|Getdecay%20time _array_element) 1.0))))))

(fn ConstructionScript)