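; AWUIPawn is a pawn that displays images received over ROS 2 on an image plate.
; On BeginPlay it initialises its node, binds the message callback to the subscriber and registers the subscription.
; Each incoming image message is converted to a texture and set as InputTexture on the plate's material.
; The callback calls CreateDynamicMaterialInstance on every message rather than caching the instance.
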(event Custom|MsgCallback
  (params (InMessage :type ROS2%20Generic%20Msg%20Object%20Reference))
  (bind _asros2img_msg (Utilities|Casting|CastToROS2ImgMsg InMessage))
  (bind _returnvalue (Class|ROS2ImgtoTexture|Convert (Class|ROS2ImgMsg|GetMsg _asros2img_msg)))
  (bind _returnvalue_2 (Rendering|Material|CreateDynamicMaterialInstance (Variables|Default|GetAWUIImagePlate) 0 0 "None" :!class /Script/Engine.PrimitiveComponent))
  (Rendering|Material|SetTextureParameterValue _returnvalue_2 "InputTexture" _returnvalue))

(event EventBeginPlay
  (bind _awuinode (Variables|Default|GetAWUINode))
  (bind _awuisubscriber (Variables|Default|GetAWUISubscriber))
  (bind _subscriber (Variables|/Script/rclUE.ROS2SubscriberComponent|GetSubscriber _awuisubscriber))
  (Class|ROS2NodeComponent|Init _awuinode)
  (Class|ROS2Subscriber|SetDelegates _subscriber (delegate Custom|MsgCallback))
  (Class|ROS2NodeComponent|AddSubscription _awuinode _subscriber))

(fn ConstructionScript)